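; Obstacle actor that traps the player in a timed typing minigame on overlap.
; When a ThirdPersonCharacter overlaps it, it picks a random word, pauses the game and shows a TypeMinigame widget.
; It stays tickable while paused so Tick can count down TimeToPlay, calling the character's DeathFunction at zero.
; The widget's TypeSuccess event stops the countdown and destroys the obstacle.
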(event `self.ReceiveTick`
  (params (DeltaSeconds :type "Float (single-precision)"))
  (if (`self.minigameActive`)
    (bind _output_get (set `self.timeToPlay` (- (`self.timeToPlay`) DeltaSeconds)))
    (if (<= _output_get 0.0)
      (bind _asthird_person_character (cast `/Game/ThirdPersonBP/Blueprints/ThirdPersonCharacter` (`GameplayStatics.GetPlayerCharacter` 0)))
      (set `self.minigameActive` false)
      (`/Game/ThirdPersonBP/Blueprints/ThirdPersonCharacter.DeathFunction` _asthird_person_character))))

(event `self.ReceiveActorBeginOverlap`
  (params (OtherActor :type "Actor Object Reference"))
  (cast `/Game/ThirdPersonBP/Blueprints/ThirdPersonCharacter` OtherActor)
  (set `self.WordToPrint` (`|GetArrayItem` (`self.Words`) (`KismetMathLibrary.RandomIntegerInRange` 0 9)))
  (`GameplayStatics.SetGamePaused` true)
  (bind _returnvalue (`|CreateWidget` "/Game/Assets/Blueprints/UI/TypeMinigame.TypeMinigame_C"))
  (`UserWidget.AddToViewport` _returnvalue 0)
  (`self.SetTickableWhenPaused` true)
  (set `self.minigameActive` true)
  (add `/Game/Assets/Blueprints/UI/TypeMinigame.TypeSuccess` _returnvalue (delegate `DestroyOnSuccess`)))

(event `DestroyOnSuccess`
  (set `self.minigameActive` false)
  (`self.K2_DestroyActor`))

(fn `UserConstructionScript`)